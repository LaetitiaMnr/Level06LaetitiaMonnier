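; BP_TypeBox is an interactable box that can be dragged and can trigger pressure plates.
; BeingDragged attaches it to the Dragger at its HandlingPoint, while BeingFree detaches it and lowers it by a release offset.
; Both events play a random grab sound from an array filled in the construction script.
; BoxMesh overlaps cast to BP_PressurePlate, calling BeingPushed on begin and BeingReleased on end.
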(event OnComponentBeginOverlap(BoxMesh)
  (params (OverlappedComponent :type Primitive%20Component%20Object%20Reference) (OtherActor :type Actor%20Object%20Reference) (OtherComp :type Primitive%20Component%20Object%20Reference) (OtherBodyIndex :type Integer) (bFromSweep :type Boolean) (SweepResult :type Hit%20Result%20Structure%20%28by%20ref%29))
  ;[1 1 1] Pressure plates interactions
  (bind _asbp_pressure_plate (Utilities|Casting|CastToBP_PressurePlate OtherActor))
  (Default|BeingPushed _asbp_pressure_plate))

(event OnComponentEndOverlap(BoxMesh)
  (params (OverlappedComponent :type Primitive%20Component%20Object%20Reference) (OtherActor :type Actor%20Object%20Reference) (OtherComp :type Primitive%20Component%20Object%20Reference) (OtherBodyIndex :type Integer))
  ;[1 1 1] Pressure plates interactions
  (bind _asbp_pressure_plate (Utilities|Casting|CastToBP_PressurePlate OtherActor))
  (Default|BeingReleased _asbp_pressure_plate))

(event Custom|BeingDragged
  (params (Dragger :type PC%20Main%20Object%20Reference))
  (bind _m_sounds (Variables|Components|GetM%20Sounds))
  (bind _audio (Variables|Default|GetAudio))
  ;[1 1 1] Attach to player
  (Audio|Components|Audio|SetSound _audio (Utilities|Array|Get(acopy) _m_sounds (Math|Random|RandomInteger (Utilities|Array|Length _m_sounds))))
  (Audio|Components|Audio|Play _audio 0.0)
  (Transformation|AttachActorToActor Dragger "None" "KeepWorld" "KeepRelative" "KeepRelative" true)
  (Transformation|SetActorLocation (Transformation|GetWorldLocation (Variables|/Game/Blueprints/Players/PC_Main.PC_Main_C|GetHandlingPoint Dragger)) false false))

(event Custom|BeingFree
  (params (Dragger :type PC%20Main%20Object%20Reference))
  (bind _returnvalue (Transformation|GetActorLocation))
  (bind _m_sounds (Variables|Components|GetM%20Sounds))
  (bind _audio (Variables|Default|GetAudio))
  ;[1 1 1] Detach from player
  (Audio|Components|Audio|SetSound _audio (Utilities|Array|Get(acopy) _m_sounds (Math|Random|RandomInteger (Utilities|Array|Length _m_sounds))))
  (Audio|Components|Audio|Play _audio 0.0)
  (Transformation|DetachFromActor "KeepWorld" "KeepWorld" "KeepRelative")
  (Transformation|SetActorTransform (Math|Transform|MakeTransform (Math|Vector|MakeVector (.x _returnvalue) (.y _returnvalue) (- (.z _returnvalue) (Variables|Components|GetM%20OffsetWhenReleased))) (Transformation|GetActorRotation))))

(fn ConstructionScript
  (|CallParentFunction)
  (Utilities|Array|Add (Variables|Components|GetM%20Sounds) "/Game/Audio/SoundEffect_GrabbingBox_Cue.SoundEffect_GrabbingBox_Cue")
  (Utilities|Array|Add (Variables|Components|GetM%20Sounds) "/Game/Audio/SoundEffect_GrabbingBox_001_Cue.SoundEffect_GrabbingBox_001_Cue")
  (Utilities|Array|Add (Variables|Components|GetM%20Sounds) "/Game/Audio/SoundEffect_GrabbingBox_002_Cue.SoundEffect_GrabbingBox_002_Cue"))