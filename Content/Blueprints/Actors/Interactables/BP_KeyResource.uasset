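; BP_KeyResource is a spinning key pickup that counts toward opening a linked door.
; When a PC_Main enters the trigger, it reports a met condition to the door, plays sound and attached sparks, removes the trigger, then destroys itself after a short delay.
; A self-restarting timeline drives the key's yaw rotation.
; The construction script assigns the achievement sound to the audio component.
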(event OnComponentBeginOverlap(Trigger)
  (params (OverlappedComponent :type Primitive%20Component%20Object%20Reference) (OtherActor :type Actor%20Object%20Reference) (OtherComp :type Primitive%20Component%20Object%20Reference) (OtherBodyIndex :type Integer) (bFromSweep :type Boolean) (SweepResult :type Hit%20Result%20Structure%20%28by%20ref%29))
  (if (== (Utilities|GetClass OtherActor) "/Game/Blueprints/Players/PC_Main.PC_Main_C")
    (Default|OneMoreCondition (Variables|Default|GetM%20LinkedDoor) 0 true)
    (Audio|Components|Audio|Play (Variables|Default|GetAudio) 0.0)
    (Effects|SpawnEmitterAttached "/Game/StarterContent/Particles/P_Sparks.P_Sparks" (Variables|Default|GetKey) "None" (Transformation|GetActorLocation) "0, 0, 0" "1.000000,1.000000,1.000000" "KeepWorldPosition")
    (Components|DestroyComponent (Variables|Default|GetTrigger))
    (Utilities|FlowControl|Delay 1.5)
    (Actor|DestroyActor)))

(event Custom|StartSpinning
  (bind _rotationvalue (Timeline|Spinning PlayFromStart)
    (:Update
      (Transformation|SetWorldRotation (Variables|Default|GetKey) (Math|Rotator|Lerp(Rotator) "0, 0, 0" (Math|Rotator|MakeRotator 0.0 0.0 (Utilities|GETROTVALUE)) _rotationvalue) false false))
    (:Finished
      (CallFunction|StartSpinning))))

(event EventBeginPlay
  (CallFunction|StartSpinning))

(event Collision|EventActorBeginOverlap
  (params (OtherActor :type Actor%20Object%20Reference)))

(fn ConstructionScript
  (|CallParentFunction)
  (Audio|Components|Audio|SetSound (Variables|Default|GetAudio) "/Game/Audio/SoundEffect_Achievement_Cue.SoundEffect_Achievement_Cue"))