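; Pressure plate interactable that starts a linked platform moving when pushed and stops it when released.
; Non-box actors trigger it by overlap, while BP_TypeBox handles its own case, and a toggle flag keeps the plate down after actors leave.
; Release waits until no boxes overlap.
; State changes play a random dragging sound, set the material and drive a Sinking timeline that lerps plate height, and ResetPlate clears the pushed state.
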(event Custom|BeingPushed
  (bind _audio (Variables|Default|GetAudio))
  (bind _m_sounds (Variables|Components|GetM%20Sounds))
  ;[1 1 1] Actions
  (if (not (Variables|States|GetM%20IsPushed))
    (Audio|Components|Audio|SetSound _audio (Utilities|Array|Get(acopy) _m_sounds (Math|Random|RandomInteger (Utilities|Array|Length _m_sounds))))
    (Audio|Components|Audio|Play _audio 0.0)
    (Rendering|Material|SetMaterial (Variables|Default|GetPlate) 0 0)
    (Default|Move (Variables|Components|GetM%20Platform))
    (Variables|States|SetM%20IsPushed true)
    (bind _zvalue (Timeline|Sinking Play)
      (:Update
        (Transformation|SetRelativeLocation (Variables|Default|GetPlate) (Math|Vector|Lerp(Vector) "0, 0, 0" (Math|Vector|MakeVector 0.0 0.0 (Utilities|GETPLATEZPOS)) _zvalue) false false)))))

(event Custom|BeingReleased
  (bind _audio (Variables|Default|GetAudio))
  (bind _m_sounds (Variables|Components|GetM%20Sounds))
  ;[1 1 1] Actions
  (if (== (Utilities|Array|Length (Collision|GetOverlappingActors "/Game/Blueprints/Actors/Interactables/BP_TypeBox.BP_TypeBox_C" :!class /Script/Engine.Actor)) 0)
    (Audio|Components|Audio|SetSound _audio (Utilities|Array|Get(acopy) _m_sounds (Math|Random|RandomInteger (Utilities|Array|Length _m_sounds))))
    (Audio|Components|Audio|Play _audio 0.0)
    (Rendering|Material|SetMaterial (Variables|Default|GetPlate) 0 0)
    (Default|Stop (Variables|Components|GetM%20Platform))
    (Variables|States|SetM%20IsPushed false)
    (bind _zvalue (Timeline|Sinking Reverse)
      (:Update
        (Transformation|SetRelativeLocation (Variables|Default|GetPlate) (Math|Vector|Lerp(Vector) "0, 0, 0" (Math|Vector|MakeVector 0.0 0.0 (Utilities|GETPLATEZPOS)) _zvalue) false false)))))

(event Collision|EventActorBeginOverlap
  (params (OtherActor :type Actor%20Object%20Reference))
  ;[1 1 1] Conditions
  (if (not (Utilities|ClassIsChildOf (Utilities|GetClass OtherActor) "/Game/Blueprints/Actors/Interactables/BP_TypeBox.BP_TypeBox_C"))
    (CallFunction|BeingPushed)))

(event Collision|EventActorEndOverlap
  (params (OtherActor :type Actor%20Object%20Reference))
  ;[1 1 1] Conditions
  ;;[0 1 0.06908] Does the plate need to be holded
  (if (not (Variables|Components|GetM%20Toggle))
    (if (not (Utilities|ClassIsChildOf (Utilities|GetClass OtherActor) "/Game/Blueprints/Actors/Interactables/BP_TypeBox.BP_TypeBox_C"))
      (CallFunction|BeingReleased))))

(fn ConstructionScript
  (bind _m_sounds (Variables|Components|GetM%20Sounds))
  (|CallParentFunction)
  (Variables|States|SetM%20IsPushed false)
  (Rendering|Material|SetMaterial (Variables|Default|GetPlate) 0 0)
  (Utilities|Array|Add _m_sounds "/Game/Audio/SoundEffect_DraggingStuff_001_Cue.SoundEffect_DraggingStuff_001_Cue")
  (Utilities|Array|Add _m_sounds "/Game/Audio/SoundEffect_DraggingStuff_002_Cue.SoundEffect_DraggingStuff_002_Cue")
  (Utilities|Array|Add _m_sounds "/Game/Audio/SoundEffect_DraggingStuff_003_Cue.SoundEffect_DraggingStuff_003_Cue")
  (Utilities|Array|Add _m_sounds "/Game/Audio/SoundEffect_DraggingStuff_004_Cue.SoundEffect_DraggingStuff_004_Cue"))

(fn ResetPlate
  (CallFunction|ResetObject)
  (Variables|States|SetM%20IsPushed false)
  (Rendering|Material|SetMaterial (Variables|Default|GetPlate) 0 0))