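; BP_Drawing is an actor that shows a pattern of up to nine nodes on a followed wall.
; On BeginPlay it attaches to the wall and its platform mesh with a relative offset, then applies a moss material to each node flagged in MNodesDatas, using a hard-coded index switch.
; The construction script adds a false entry to MNodesStates for each child of the root component.
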(event EventBeginPlay
  (Transformation|AttachActorToActor (Variables|Default|GetM%20FollowedWall) "None" "KeepRelative" "KeepRelative" "KeepRelative" true)
  (Transformation|SetActorRelativeLocation "50.000000, 0, 0")
  (Transformation|AttachComponentToComponent (Variables|/Game/Blueprints/Actors/Architectures/BP_TypePlatform.BP_TypePlatform_C|GetPlatformMesh (Variables|Default|GetM%20FollowedWall)) "None" "KeepRelative" "KeepRelative" "KeepRelative" true)
  (for (_array_element _array_index) (Variables|Components|GetM%20NodesDatas)
    (if _array_element
      ;[1 1 1] Awful code, don't watch this.
      (switch int _array_index
        (:0
          (CallFunction|SetMaterial (Variables|Default|GetNode)))
        (:1
          (CallFunction|SetMaterial (Variables|Default|GetNode1)))
        (:2
          (CallFunction|SetMaterial (Variables|Default|GetNode2)))
        (:3
          (CallFunction|SetMaterial (Variables|Default|GetNode3)))
        (:4
          (CallFunction|SetMaterial (Variables|Default|GetNode4)))
        (:5
          (CallFunction|SetMaterial (Variables|Default|GetNode5)))
        (:6
          (CallFunction|SetMaterial (Variables|Default|GetNode6)))
        (:7
          (CallFunction|SetMaterial (Variables|Default|GetNode7)))
        (:8
          (CallFunction|SetMaterial (Variables|Default|GetNode8)))))))

(fn ConstructionScript
  (for _array_element (Components|GetChildrenComponents (Variables|Default|GetDefaultSceneRoot self) false)
    (Utilities|Array|Add (Variables|Components|GetM%20NodesStates) false)))

(fn SetMaterial
  (params (SMC :type Static%20Mesh%20Component%20Object%20Reference%20%28by%20ref%29))
  (Rendering|Material|SetMaterial SMC 0 "/Game/StarterContent/Materials/M_Ground_Moss.M_Ground_Moss"))