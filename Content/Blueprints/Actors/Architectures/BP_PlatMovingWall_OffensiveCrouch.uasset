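; BP_PlatMovingWall_OffensiveCrouch is a moving wall platform variant that uses a full-wall mesh with a crouch hole.
; The construction script runs the parent's logic, then applies that mesh and a default timeline play rate to the inherited platform components.
; After the parent's BeginPlay, a nonzero MTimelinePlayRate overrides the animation speed and a valid MWallMesh replaces the mesh.
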(event EventBeginPlay
  (|CallParentFunction)
  (if (!= 0.0 (Variables|Default|GetM%20TimelinePlayRate))
    (Components|Timeline|SetPlayRate (Variables|Default|GetPlatformAnimation) (Variables|Default|GetM%20TimelinePlayRate)))
  (if (Utilities|IsValid (Variables|Default|GetM%20WallMesh))
    (Components|StaticMesh|SetStaticMesh (Variables|Default|GetPlatformMesh) (Variables|Default|GetM%20WallMesh))))

(fn ConstructionScript
  (|CallParentFunction)
  ;[1 1 1] Default values
  (Components|StaticMesh|SetStaticMesh (Variables|Default|GetPlatformMesh) "/Game/Meshes/Walls/SM_WallFull_CrouchHole.SM_WallFull_CrouchHole")
  (Components|Timeline|SetPlayRate (Variables|Default|GetPlatformAnimation) 1.125))