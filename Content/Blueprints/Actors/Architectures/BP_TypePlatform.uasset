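; Moving platform actor that oscillates back and forth along a vertical or horizontal axis, with optional tangibility switching.
; On BeginPlay it optionally starts, after an optional delay, a timeline that lerps the mesh's relative location and alternates Play and Reverse.
; Tangible mode drives a dynamic material color from the timeline and toggles collision at the far end and midway back.
; A helper stops a platform and restores its starting transform.
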(event Custom|Move
  ;[1 1 1] Animations
  ;;[0 1 0.05672] Tangibility variable
  (Variables|Components|SetM%20Switched false)
  (bind (_direction _force _colortangibility) (Timeline|PlatformAnimation Play)
    (:Update
      (if (Variables|Ajust|GetM%20Tang)
        (if (Math|Boolean|ANDBoolean (Utilities|IsTimelineatHalfReverse (Variables|Default|GetPlatformAnimation)) (not (Variables|Movement|GetM%20MoveForward)) (not (Variables|Components|GetM%20Switched)))
          (CallFunction|SetOppositeCollisions (Variables|Default|GetPlatformMesh))
          (Variables|Components|SetM%20Switched true)))
      (if (Variables|Movement|GetM%20Vertical)
        (Transformation|SetRelativeLocation (Variables|Default|GetPlatformMesh) (Math|Vector|Lerp(Vector) "0, 0, 0" (Math|Vector|MakeVector 0.0 0.0 (Variables|Ajust|GetM%20AxisDestination)) _force) false false)
        (else
          (Transformation|SetRelativeLocation (Variables|Default|GetPlatformMesh) (Math|Vector|Lerp(Vector) "0, 0, 0" (Math|Vector|MakeVector (Variables|Ajust|GetM%20AxisDestination) 0.0 0.0) _force) false false)))
      (if (Variables|Ajust|GetM%20Tang)
        (Rendering|Material|SetVectorParameterValue (Variables|Components|GetM%20DynamicMaterial) "Color" _colortangibility :!class /Script/Engine.MaterialInstanceDynamic)))
    (:Finished
      ;;[1 1 1] Resetting states
      (bind _output_get (Variables|Movement|SetM%20MoveForward (not (Variables|Movement|GetM%20MoveForward))))
      (if (and (Variables|Ajust|GetM%20Tang) (not (Variables|Movement|GetM%20MoveForward)))
        (CallFunction|SetOppositeCollisions (Variables|Default|GetPlatformMesh)))
      (if _output_get
        (CallFunction|Move)
        (else
          (CallFunction|Reverse))))))

(event Custom|MoveFromStart
  ;[1 1 1] Animations
  ;;[0 1 0.05672] Tangibility variable
  (Variables|Components|SetM%20Switched false)
  (bind (_direction _force _colortangibility) (Timeline|PlatformAnimation PlayFromStart)
    (:Update
      (if (Variables|Ajust|GetM%20Tang)
        (if (Math|Boolean|ANDBoolean (Utilities|IsTimelineatHalfReverse (Variables|Default|GetPlatformAnimation)) (not (Variables|Movement|GetM%20MoveForward)) (not (Variables|Components|GetM%20Switched)))
          (CallFunction|SetOppositeCollisions (Variables|Default|GetPlatformMesh))
          (Variables|Components|SetM%20Switched true)))
      (if (Variables|Movement|GetM%20Vertical)
        (Transformation|SetRelativeLocation (Variables|Default|GetPlatformMesh) (Math|Vector|Lerp(Vector) "0, 0, 0" (Math|Vector|MakeVector 0.0 0.0 (Variables|Ajust|GetM%20AxisDestination)) _force) false false)
        (else
          (Transformation|SetRelativeLocation (Variables|Default|GetPlatformMesh) (Math|Vector|Lerp(Vector) "0, 0, 0" (Math|Vector|MakeVector (Variables|Ajust|GetM%20AxisDestination) 0.0 0.0) _force) false false)))
      (if (Variables|Ajust|GetM%20Tang)
        (Rendering|Material|SetVectorParameterValue (Variables|Components|GetM%20DynamicMaterial) "Color" _colortangibility :!class /Script/Engine.MaterialInstanceDynamic)))
    (:Finished
      ;;[1 1 1] Resetting states
      (bind _output_get (Variables|Movement|SetM%20MoveForward (not (Variables|Movement|GetM%20MoveForward))))
      (if (and (Variables|Ajust|GetM%20Tang) (not (Variables|Movement|GetM%20MoveForward)))
        (CallFunction|SetOppositeCollisions (Variables|Default|GetPlatformMesh)))
      (if _output_get
        (CallFunction|Move)
        (else
          (CallFunction|Reverse))))))

(event Custom|Reverse
  ;[1 1 1] Animations
  ;;[0 1 0.05672] Tangibility variable
  (Variables|Components|SetM%20Switched false)
  (bind (_direction _force _colortangibility) (Timeline|PlatformAnimation Reverse)
    (:Update
      (if (Variables|Ajust|GetM%20Tang)
        (if (Math|Boolean|ANDBoolean (Utilities|IsTimelineatHalfReverse (Variables|Default|GetPlatformAnimation)) (not (Variables|Movement|GetM%20MoveForward)) (not (Variables|Components|GetM%20Switched)))
          (CallFunction|SetOppositeCollisions (Variables|Default|GetPlatformMesh))
          (Variables|Components|SetM%20Switched true)))
      (if (Variables|Movement|GetM%20Vertical)
        (Transformation|SetRelativeLocation (Variables|Default|GetPlatformMesh) (Math|Vector|Lerp(Vector) "0, 0, 0" (Math|Vector|MakeVector 0.0 0.0 (Variables|Ajust|GetM%20AxisDestination)) _force) false false)
        (else
          (Transformation|SetRelativeLocation (Variables|Default|GetPlatformMesh) (Math|Vector|Lerp(Vector) "0, 0, 0" (Math|Vector|MakeVector (Variables|Ajust|GetM%20AxisDestination) 0.0 0.0) _force) false false)))
      (if (Variables|Ajust|GetM%20Tang)
        (Rendering|Material|SetVectorParameterValue (Variables|Components|GetM%20DynamicMaterial) "Color" _colortangibility :!class /Script/Engine.MaterialInstanceDynamic)))
    (:Finished
      ;;[1 1 1] Resetting states
      (bind _output_get (Variables|Movement|SetM%20MoveForward (not (Variables|Movement|GetM%20MoveForward))))
      (if (and (Variables|Ajust|GetM%20Tang) (not (Variables|Movement|GetM%20MoveForward)))
        (CallFunction|SetOppositeCollisions (Variables|Default|GetPlatformMesh)))
      (if _output_get
        (CallFunction|Move)
        (else
          (CallFunction|Reverse))))))

(event Custom|Stop
  ;[1 1 1] Animations
  (bind (_direction _force _colortangibility) (Timeline|PlatformAnimation Stop)
    (:Update
      (if (Variables|Ajust|GetM%20Tang)
        (if (Math|Boolean|ANDBoolean (Utilities|IsTimelineatHalfReverse (Variables|Default|GetPlatformAnimation)) (not (Variables|Movement|GetM%20MoveForward)) (not (Variables|Components|GetM%20Switched)))
          (CallFunction|SetOppositeCollisions (Variables|Default|GetPlatformMesh))
          (Variables|Components|SetM%20Switched true)))
      (if (Variables|Movement|GetM%20Vertical)
        (Transformation|SetRelativeLocation (Variables|Default|GetPlatformMesh) (Math|Vector|Lerp(Vector) "0, 0, 0" (Math|Vector|MakeVector 0.0 0.0 (Variables|Ajust|GetM%20AxisDestination)) _force) false false)
        (else
          (Transformation|SetRelativeLocation (Variables|Default|GetPlatformMesh) (Math|Vector|Lerp(Vector) "0, 0, 0" (Math|Vector|MakeVector (Variables|Ajust|GetM%20AxisDestination) 0.0 0.0) _force) false false)))
      (if (Variables|Ajust|GetM%20Tang)
        (Rendering|Material|SetVectorParameterValue (Variables|Components|GetM%20DynamicMaterial) "Color" _colortangibility :!class /Script/Engine.MaterialInstanceDynamic)))
    (:Finished
      ;;[1 1 1] Resetting states
      (bind _output_get (Variables|Movement|SetM%20MoveForward (not (Variables|Movement|GetM%20MoveForward))))
      (if (and (Variables|Ajust|GetM%20Tang) (not (Variables|Movement|GetM%20MoveForward)))
        (CallFunction|SetOppositeCollisions (Variables|Default|GetPlatformMesh)))
      (if _output_get
        (CallFunction|Move)
        (else
          (CallFunction|Reverse))))))

(event Custom|Init
  ;[1 1 1] Default call
  (if (Variables|Ajust|GetM%20Tang)
    (bind _returnvalue (Rendering|Material|CreateDynamicMaterialInstance (Variables|Default|GetPlatformMesh) 1 0 :!class /Script/Engine.PrimitiveComponent))
    (Variables|Components|SetM%20DynamicMaterial _returnvalue))
  (if (Variables|Movement|GetM%20BeginMove)
    (if (> (Utilities|NearestTenth (Variables|Ajust|GetM%20InvokeDelay)) 0.0)
      (Utilities|FlowControl|Delay (Variables|Ajust|GetM%20InvokeDelay)))
    (CallFunction|Move)))

(event EventBeginPlay
  ;[1 1 1] Default call
  (CallFunction|Init))

(fn ConstructionScript
  (Variables|Movement|SetM%20MoveForward true)
  (Variables|Components|SetM%20Switched false)
  (Variables|Components|SetM%20StartTransform (Transformation|GetWorldTransform (Variables|Default|GetPlatformMesh)))
  (Variables|Components|SetM%20StartPlatformTransform (Transformation|GetActorTransform self)))

(fn SetOppositeCollisions
  (params (Mesh :type Primitive%20Component%20Object%20Reference%20%28by%20ref%29))
  (switch Utilities|FlowControl|Switch|SwitchonECollisionEnabled (Collision|GetCollisionEnabled Mesh)
    (:NoCollision
      (Collision|SetCollisionEnabled Mesh "QueryAndPhysics"))
    (:QueryAndPhysics
      (Collision|SetCollisionEnabled Mesh "NoCollision"))))

(fn MeshBacktoStart
  (params (Platform :type BP%20Type%20Platform%20Object%20Reference))
  (CallFunction|Stop Platform)
  (Transformation|SetWorldTransform (Variables|BP_TypePlatform_C|GetPlatformMesh Platform) (Variables|BP_TypePlatform_C|GetM%20StartTransform Platform) false false)
  (Variables|Components|SetM%20Switched false)
  (Variables|Movement|SetM%20MoveForward true))