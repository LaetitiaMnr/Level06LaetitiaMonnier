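; Moving wall platform that shoves the player along its forward vector and crushes them against offensive walls.
; Extends parent platform movement with Z correction, looping-agnostic audio and push strength derived from animation play rate; Reverse is disabled.
; Trigger overlaps drive a Tick-fed gate for pushing.
; Destroyable actors and offensive walls hit without a player inside are fake-destroyed by moving them to world origin, with platforms first passed to MeshBackToStart.
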(event OnComponentBeginOverlap(Trigger)
  (params (OverlappedComponent :type Primitive%20Component%20Object%20Reference) (OtherActor :type Actor%20Object%20Reference) (OtherComp :type Primitive%20Component%20Object%20Reference) (OtherBodyIndex :type Integer) (bFromSweep :type Boolean) (SweepResult :type Hit%20Result%20Structure%20%28by%20ref%29))
  (bind _trigger (Variables|Default|GetTrigger))
  (bind _overlappingactors (Collision|GetOverlappingActors _trigger 0 :!class /Script/Engine.PrimitiveComponent))
  ;[1 1 1] SUPPOSED TO ... Push back objects excluding other walls (in this case, it "destroys" them)
  (if (Utilities|IsOffensiveWall OtherActor)
    (bind _return (CallFunction|PlayerInside _overlappingactors))
    (if (> _return -1)
      (bind _aspc_main (Utilities|Casting|CastToPC_Main (Utilities|Array|Get(acopy) _overlappingactors _return)))
      (Default|Death _aspc_main "crush")
      (else
        (bind _asbp_type_platform (Utilities|Casting|CastToBP_TypePlatform OtherActor)
          (:then
            (CallFunction|MeshBacktoStart _asbp_type_platform))
          (:CastFailed
            _))
        (CallFunction|SimulateDestroy _asbp_type_platform)))
    (elif (Utilities|IsDestroyable OtherActor)
      (CallFunction|SimulateDestroy OtherActor)
      (elif (Utilities|IsPlayer OtherActor)
        (Utilities|FlowControl|Gate true) ; enters at Open
      ))))

(event OnComponentEndOverlap(Trigger)
  (params (OverlappedComponent :type Primitive%20Component%20Object%20Reference) (OtherActor :type Actor%20Object%20Reference) (OtherComp :type Primitive%20Component%20Object%20Reference) (OtherBodyIndex :type Integer))
  ;[1 1 1] SUPPOSED TO ... Push back objects excluding other walls (in this case, it "destroys" them)
  (if (Utilities|IsPlayer OtherActor)
    (Utilities|FlowControl|Gate true) ; enters at Close
    (elif (not (Utilities|IsTriggerEvent OtherActor))
      (Audio|SpawnSoundatLocation "/Game/StarterContent/Audio/Collapse_Cue.Collapse_Cue" (Transformation|GetActorLocation)))))

(event EventMovefromStart
  ;[1 1 1] Add extra values to the parent move and stop function
  (|CallParentFunction)
  (if true
    (CallFunction|MovetoProperZLocation (Transformation|GetActorLocation))
    (Variables|Effects|SetM%20PushingDirectionMultiplier (* (Components|Animation|GetPlayRate (Variables|Default|GetPlatformAnimation)) 1e+01))
    (Audio|Components|Audio|Play (Variables|Default|GetMovingAudio) 0.0)))

(event EventMove
  ;[1 1 1] Add extra values to the parent move and stop function
  (|CallParentFunction)
  (if true
    (CallFunction|MovetoProperZLocation (Transformation|GetActorLocation))
    (Variables|Effects|SetM%20PushingDirectionMultiplier (* (Components|Animation|GetPlayRate (Variables|Default|GetPlatformAnimation)) 1e+01))
    (Audio|Components|Audio|Play (Variables|Default|GetMovingAudio) 0.0)))

(event EventReverse
  ;[0 1 0.05504] Override parent function (When Reverse is called, nothing should happen)
)

(event EventTick
  (params (DeltaSeconds :type Float%20%28single-precision%29))
  ;[1 1 1] SUPPOSED TO ... Push back objects excluding other walls (in this case, it "destroys" them)
  (Utilities|FlowControl|Gate true
    (:Exit
      (Transformation|AddActorWorldOffset (stale OnComponentBeginOverlap(Trigger) OtherActor) (* (Transformation|GetActorForwardVector) (Variables|Effects|GetM%20PushingDirectionMultiplier))))))

(event EventStop
  ;[1 1 1] Add extra values to the parent move and stop function
  (|CallParentFunction)
  (Audio|Components|Audio|Stop (Variables|Default|GetMovingAudio)))

(fn ConstructionScript
  (|CallParentFunction)
  (Components|StaticMesh|SetStaticMesh (Variables|Default|GetPlatformMesh) "/Game/Meshes/Walls/SM_WallFull_Filled.SM_WallFull_Filled")
  ;[1 1 1] Default values
  (Components|Timeline|SetPlayRate (Variables|Default|GetPlatformAnimation) 0.25)
  (Variables|Effects|SetM%20PushingDirectionMultiplier 1.0)
  (Audio|Components|Audio|SetSound (Variables|Default|GetMovingAudio) "/Game/Audio/SoundEffect_ElevatorFalling_Cue.SoundEffect_ElevatorFalling_Cue"))

(fn MovetoProperZLocation
  (params (CurrentPosition :type Vector))
  (Transformation|SetActorLocation (Math|Vector|MakeVector (.x CurrentPosition) (.y CurrentPosition) (Utilities|GETZPROPERLOCATION)) false false))

(fn SimulateDestroy
  (params (Actor :type Actor%20Object%20Reference%20%28by%20ref%29))
  (Transformation|SetActorLocation Actor "0, 0, 0" false false))

(fn PlayerInside
  (params (Array :type Array%20of%20Actor%20Object%20References))
  (for (_array_element _array_index) Array
    (if (.bSuccess (Utilities|Casting|CastToPC_Main _array_element))
      (return _array_index)))
  (return -1))