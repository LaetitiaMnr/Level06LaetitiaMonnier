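; HUD_Main is the main HUD, which shows the player's on-screen prompts and checkpoint feedback.
; On BeginPlay it creates a WBP_Main widget for the first player controller, stores it and adds it to the viewport.
; Its Interact, Drag and Checkpoint events act as a thin relay, forwarding calls and their show and key arguments to the matching widget functions.
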(event Custom|Interact
  (params (Show :type Boolean) (Key :type Key%20Structure))
  (Default|InteractImage (Variables|Components|GetM%20MainWidget) Show Key))

(event Custom|Checkpoint
  (Default|Checkpoint (Variables|Components|GetM%20MainWidget)))

(event Custom|Drag
  (params (Show :type Boolean) (Key :type Key%20Structure))
  (Default|DragImage (Variables|Components|GetM%20MainWidget) Show Key))

(event EventBeginPlay
  (bind _returnvalue (UserInterface|CreateWidget "/Game/Blueprints/Widgets/WBP_Main.WBP_Main_C" (Game|GetPlayerController 0)))
  (bind _output_get (Variables|Components|SetM%20MainWidget _returnvalue))
  (UserInterface|Viewport|AddtoViewport _output_get 0))

(fn ConstructionScript)