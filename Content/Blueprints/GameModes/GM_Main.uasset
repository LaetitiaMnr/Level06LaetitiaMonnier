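; Main game mode that handles checkpoints, player respawning and resetting of level actors.
; NewCheckpoint stores the position and notifies HUD_Main, and Respawn spawns a fresh PC_Main there for the first player controller to possess.
; A separate ResetActors event finds every door, object and platform by class and resets it, returning platforms to their starting transform and re-initializing them.
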(event Custom|Respawn
  (bind _returnvalue (Game|SpawnActorfromClass "/Game/Blueprints/Players/PC_Main.PC_Main_C" (Math|Transform|MakeTransform (Variables|Components|GetM%20CurrentCheckPoint) "0.000000,180.000000, 0") "Undefined" 0 0))
  (Pawn|Possess (Game|GetPlayerController 0) _returnvalue))

(event Custom|ResetActors
  (CallFunction|ResetAllDoors)
  (CallFunction|ResetAllObjects)
  (CallFunction|ResetAllPlatforms))

(fn ConstructionScript)

(fn NewCheckpoint
  (params (CheckpointPosition :type Vector) (PlayerController :type Player%20Controller%20Object%20Reference))
  (Variables|Components|SetM%20CurrentCheckPoint CheckpointPosition)
  (bind _ashud_main (Utilities|Casting|CastToHUD_Main (HUD|GetHUD (Game|GetPlayerController 0))))
  (Default|Checkpoint _ashud_main))

(fn ResetAllObjects
  (bind _outactors (Actor|GetAllActorsOfClass "/Game/Blueprints/Actors/Interactables/BP_Object.BP_Object_C"))
  (for _array_element _outactors
    (Default|ResetObject _array_element)))

(fn ResetAllDoors
  (bind _outactors (Actor|GetAllActorsOfClass "/Game/Blueprints/Actors/Architectures/BP_Door.BP_Door_C"))
  (for _array_element _outactors
    (Default|ResetDoor _array_element)))

(fn ResetAllPlatforms
  (bind _outactors (Actor|GetAllActorsOfClass "/Game/Blueprints/Actors/Architectures/BP_TypePlatform.BP_TypePlatform_C"))
  (for _array_element _outactors
    (Transformation|SetActorTransform _array_element (Variables|/Game/Blueprints/Actors/Architectures/BP_TypePlatform.BP_TypePlatform_C|GetM%20StartPlatformTransform _array_element))
    (Default|MeshBacktoStart _array_element _array_element)
    (Default|Init _array_element)))